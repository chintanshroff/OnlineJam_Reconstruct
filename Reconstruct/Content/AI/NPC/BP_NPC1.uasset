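; Enemy NPC for a top-down game that melee-attacks the player and displays its field of view as a mesh on the ground plane.
; MeleeAttack plays an attack montage, during which weapon overlaps kill a living player.
; Every Tick runs an EQS VisionCone query, whose points become a triangle fan rebuilt on a procedural mesh.
; KillAI marks it dead, disables movement and turns on mesh physics simulation.
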(event `/Game/CombatInterface.MeleeAttack`
  ;[1 1 1] DoMeleeAttack
  (if (not (`self.isDead`))
    (bind _astop_down_character (cast `/Game/TopDownBP/Blueprints/TopDownCharacter` (`GameplayStatics.GetPlayerCharacter` 0)))
    (if (not (`/Game/TopDownBP/Blueprints/TopDownCharacter.isDead` _astop_down_character))
      (`|PlayMontage` (`self.Mesh`) "/Game/AI/NPC/Attack_PrimaryA_NPC_Montage_NPC.Attack_PrimaryA_NPC_Montage_NPC"
        (:`then`
          (set `self.isHitting` true))
        (:`OnCompleted`
          (set `self.isHitting` false))))))

(event `self.Weapon.OnComponentBeginOverlap`
  (params (OverlappedComponent :type "PrimitiveComponent Object Reference") (OtherActor :type "Actor Object Reference") (OtherComp :type "PrimitiveComponent Object Reference") (OtherBodyIndex :type Integer) (bFromSweep :type Boolean) (SweepResult :type "HitResult Structure (by ref)"))
  ;[1 1 1] Check If Player dead
  (if (== (`GameplayStatics.GetObjectClass` OtherActor) "/Game/TopDownBP/Blueprints/TopDownCharacter.TopDownCharacter_C")
    (bind _astop_down_character (cast `/Game/TopDownBP/Blueprints/TopDownCharacter` OtherActor))
    (if (and (not (`/Game/TopDownBP/Blueprints/TopDownCharacter.isDead` _astop_down_character)) (`self.isHitting`))
      (`/Game/TopDownBP/Blueprints/TopDownCharacter.KillPlayer` _astop_down_character))))

(event `self.ReceiveBeginPlay`
  (`KismetArrayLibrary.Array_Resize` (`self.Vertices`) 51))

(event `self.ReceiveTick`
  (params (DeltaSeconds :type "Float (single-precision)"))
  (bind _returnvalue (`EnvQueryManager.RunEQSQuery` "/Game/AI/VisionConeStuff/VisionCone.VisionCone" self "AllMatching"))
  (add `EnvQueryInstanceBlueprintWrapper.OnQueryFinishedEvent` _returnvalue (delegate `MakeMyCone`)))

(event `MakeMyCone`
  (params (QueryInstance :type "EnvQueryInstanceBlueprintWrapper Object Reference") (QueryStatus :type "EEnvQueryStatus Enum" :default "Processing"))
  (bind _resultlocations (`EnvQueryInstanceBlueprintWrapper.GetQueryResultsAsLocations` QueryInstance))
  (bind _output_get (set `self.SightPoints` _resultlocations))
  (bind (_vertices _triangles) (`self.ConvertSightPointsToVertices` _output_get))
  (`self.MakeTheCone` _vertices _triangles))

(fn `ConvertSightPointsToVertices`
  (params (SightPoints :type "Array of Vector Structure"))
  (returns (Vertices :type "Array of Vector Structure") (Triangles :type "Array of Integer"))
  (bind _returnvalue (`KismetArrayLibrary.Array_Length` (`self.Vertices`)))
  (`KismetArrayLibrary.Array_Set` (`self.Vertices`))
  (for (_array_element _array_index) SightPoints
    (`KismetArrayLibrary.Array_Set` (`self.Vertices`) (+ _array_index 1) (`KismetMathLibrary.MakeVector` (- (.x _array_element) (.x (`self.K2_GetActorLocation`))) (- (.y _array_element) (.y (`self.K2_GetActorLocation`))))))
  (`KismetArrayLibrary.Array_Resize` (`self.Traingles`) _returnvalue)
  (for _index (range (+ _returnvalue 1))
    (bind _returnvalue_2 (* _index 3))
    (`KismetArrayLibrary.Array_Set` (`self.Traingles`) _returnvalue_2)
    (bind _returnvalue_3 (+ _index 1))
    (`KismetArrayLibrary.Array_Set` (`self.Traingles`) 0 _returnvalue_3)
    (`KismetArrayLibrary.Array_Set` (`self.Traingles`) (+ (+ _returnvalue_2 1) 1) (+ _returnvalue_3 1)))
  (return (`self.Vertices`) (`self.Traingles`)))

(fn `KillAI`
  (bind _mesh (`self.Mesh`))
  (set `self.isDead` true)
  (`CharacterMovementComponent.DisableMovement` (`self.CharacterMovement`))
  (`PrimitiveComponent.SetCollisionEnabled` _mesh "QueryAndPhysics")
  (`SkeletalMeshComponent.SetAllBodiesSimulatePhysics` _mesh true)
  (`SkeletalMeshComponent.SetAllBodiesPhysicsBlendWeight` _mesh 0.0 false))

(fn `MakeTheCone`
  (params (Vertices :type "Array of Vector Structure") (Triangles :type "Array of Integer"))
  (bind _visioncone (`self.VisionCone`))
  (`ProceduralMeshComponent.CreateMeshSection_LinearColor` :`self` _visioncone :`Vertices` Vertices :`Triangles` Triangles)
  (`PrimitiveComponent.SetMaterial` _visioncone 0 "/Game/TopDownBP/Blueprints/M_GhostTrails.M_GhostTrails")
  (`SceneComponent.K2_SetWorldRotation` :`self` _visioncone))

(fn `UserConstructionScript`)