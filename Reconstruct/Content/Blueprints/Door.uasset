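; Door Blueprint that slides open when something overlaps its trigger, then closes itself after a short hold.
; A status enum (Closed, Opening, Open, Closing) gates each step, and two timelines drive the door component's relative location to open and close it.
; An overlap during closing waits briefly, marks the door closed, and replays the opening timeline from the start.
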(event `self.Trigger.OnComponentBeginOverlap`
  (params (OverlappedComponent :type "PrimitiveComponent Object Reference") (OtherActor :type "Actor Object Reference") (OtherComp :type "PrimitiveComponent Object Reference") (OtherBodyIndex :type Integer) (bFromSweep :type Boolean) (SweepResult :type "HitResult Structure (by ref)"))
  (switch `/Game/DoorStatus` (`self.Status`)
    (:`NewEnumerator0`
      (bind (_direction _doorlocation) (`Timeline|OpenDOor` :!via `PlayFromStart` :!label _label)
        (:`Update`
          (set `self.Status` "NewEnumerator1")
          (`SceneComponent.K2_SetRelativeLocation` (`self.Door`) _doorlocation false false))
        (:`Finished`
          (set `self.Status` "NewEnumerator2")
          (`KismetSystemLibrary.Delay` 1.0)
          (switch `/Game/DoorStatus` (`self.Status`)
            (:`NewEnumerator2`
              (bind (_direction_2 _doorlocation_2) (`Timeline|CloseDoor` :`NewTime` 0.0 :!via `PlayFromStart`)
                (:`Update`
                  (set `self.Status` "NewEnumerator3")
                  (`SceneComponent.K2_SetRelativeLocation` (`self.Door`) _doorlocation_2 false false))
                (:`Finished`
                  (set `self.Status` "NewEnumerator0"))))))))
    (:`NewEnumerator3`
      (`KismetSystemLibrary.Delay` 0.5)
      (set `self.Status` "NewEnumerator0")
      (goto _label :!via `PlayFromStart`))))

(fn `UserConstructionScript`)