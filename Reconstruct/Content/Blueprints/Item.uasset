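; Base item actor with a mesh that acts as a weapon against BP_NPC1 enemies.
; When the root component activates, the mesh takes its mass from the item structure.
; A mesh overlap with a BP_NPC1 while player 0's TopDownCharacter is hitting increments and prints a hit counter, then calls KillAI on that NPC.
; The Interact event is an empty stub.
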(event `Interact`)

(event `self.DefaultSceneRoot.OnComponentActivated`
  (params (Component :type "ActorComponent Object Reference") (bReset :type Boolean))
  (bind (_itemstructure_name _itemstructure_hitsbeforedestroy _itemstructure_class _itemstructure_mass) (break `/Game/Blueprints/ItemStructure` (`self.ItemStructure`)))
  (`PrimitiveComponent.SetMassOverrideInKg` (`self.ItemMesh`) "None" _itemstructure_mass true))

(event `self.ItemMesh.OnComponentBeginOverlap`
  (params (OverlappedComponent :type "PrimitiveComponent Object Reference") (OtherActor :type "Actor Object Reference") (OtherComp :type "PrimitiveComponent Object Reference") (OtherBodyIndex :type Integer) (bFromSweep :type Boolean) (SweepResult :type "HitResult Structure (by ref)"))
  (bind _astop_down_character (cast `/Game/TopDownBP/Blueprints/TopDownCharacter` (`GameplayStatics.GetPlayerCharacter` 0)))
  (if (and (== (`GameplayStatics.GetObjectClass` OtherActor) "/Game/AI/NPC/BP_NPC1.BP_NPC1_C") (`/Game/TopDownBP/Blueprints/TopDownCharacter.isHitting` _astop_down_character))
    (bind _result (`/Engine/EditorBlueprintResources/StandardMacros.IncrementInt` (`self.hits`))
      (:`  `
        (`KismetSystemLibrary.PrintString` (`KismetStringLibrary.Conv_IntToString` _result))
        (bind _asbp_npc1 (cast `/Game/AI/NPC/BP_NPC1` OtherActor))
        (`/Game/AI/NPC/BP_NPC1.KillAI` _asbp_npc1)))))

(fn `UserConstructionScript`)